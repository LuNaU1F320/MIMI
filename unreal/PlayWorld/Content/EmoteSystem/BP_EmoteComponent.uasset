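; BP_EmoteComponent is a scene-based component in the emote system that turns itself to face the local player's camera, billboard style.
; BeginPlay caches the camera manager of player controller 0 after validity checks.
; Every Tick it sets its world rotation to a look-at from its own location to the camera manager's location, without rechecking that the cached reference is valid.
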(event `self.ReceiveBeginPlay`
  (bind _returnvalue (`GameplayStatics.GetPlayerController` 0))
  (bind _playercameramanager (`PlayerController.PlayerCameraManager` _returnvalue))
  (`/Engine/EditorBlueprintResources/StandardMacros.IsValid` _returnvalue
    (:`Is Valid`
      (`/Engine/EditorBlueprintResources/StandardMacros.IsValid` _playercameramanager
        (:`Is Valid`
          (set `self.Player Camera Manager` _playercameramanager))))))

(event `self.ReceiveTick`
  (params (DeltaSeconds :type "Float (single-precision)"))
  (`self.K2_SetWorldRotation` (`KismetMathLibrary.FindLookAtRotation` (`self.K2_GetComponentLocation`) (`Actor.K2_GetActorLocation` (`self.Player Camera Manager`)))))